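; Player Blueprint for a ball game that records its start point and removes itself after falling out of the world.
; On BeginPlay it writes its transform to the HoleinGameMode as the SpawnTransform.
; Each Tick it checks the world height of its Ball component and destroys the actor once it drops far below the level.
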(event `self.ReceiveBeginPlay`
  (bind _asholein_game_mode (cast `/Game/Setting/HoleinGameMode` (`GameplayStatics.GetGameMode`)))
  (set `/Game/Setting/HoleinGameMode.Spawn Transform` (`self.GetTransform`) _asholein_game_mode))

(event `self.ReceiveTick`
  (params (DeltaSeconds :type "Float (single-precision)"))
  (if (< (.z (`SceneComponent.K2_GetComponentLocation` (`self.Ball`))) -10000.0)
    (`self.K2_DestroyActor`)))

(event `self.ReceiveActorBeginOverlap`
  (params (OtherActor :type "Actor Object Reference")))

(fn `UserConstructionScript`)