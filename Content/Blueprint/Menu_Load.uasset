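; Menu_Load is a menu actor whose Execute event opens a level named from Holein_SaveGame progress fields.
; It joins ClearedWorld, an underscore and ClearedLevel plus one into the level name.
; Those fields come from a newly created save game object rather than a loaded slot, so they hold class defaults.
; BeginPlay, Tick and the construction script only call their parent versions.
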(event `self.ReceiveBeginPlay`
  (`parent.ReceiveBeginPlay`))

(event `self.ReceiveActorBeginOverlap`
  (params (OtherActor :type "Actor Object Reference")))

(event `self.ReceiveTick`
  (params (DeltaSeconds :type "Float (single-precision)"))
  (`parent.ReceiveTick` DeltaSeconds))

(event `self.Execute`
  (bind _returnvalue (`GameplayStatics.CreateSaveGameObject` "/Game/Setting/Holein_SaveGame.Holein_SaveGame_C"))
  (bind _asholein_save_game (cast `/Game/Setting/Holein_SaveGame` _returnvalue))
  (`GameplayStatics.OpenLevel` (`KismetStringLibrary.Conv_StringToName` (`KismetStringLibrary.Concat_StrStr` (`/Game/Setting/Holein_SaveGame.Cleared World` _asholein_save_game) "_" (`KismetStringLibrary.Conv_IntToString` (+ (`KismetStringLibrary.Conv_StringToInt` (`/Game/Setting/Holein_SaveGame.Cleared Level` _asholein_save_game)) 1))))))

(fn `UserConstructionScript`
  (`parent.UserConstructionScript`))