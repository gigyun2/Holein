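; Menu actor with a gauge that fills through Add calls and triggers Execute when full, likely a base for selectable menu items.
; Throttled Tick drains Percentage whenever it is unchanged since the last update, so the gauge falls back without repeated Add calls.
; The value drives a "Percentage" scalar on the Graph component's dynamic material.
; Execute is an empty stub, called on each update while full.
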(event `self.ReceiveBeginPlay`
  (bind _returnvalue (`PrimitiveComponent.CreateDynamicMaterialInstance` (`self.Graph`) 0 null))
  (set `self.Gauge_Instance` _returnvalue))

(event `self.ReceiveActorBeginOverlap`
  (params (OtherActor :type "Actor Object Reference")))

(event `self.ReceiveTick`
  (params (DeltaSeconds :type "Float (single-precision)"))
  (bind _returnvalue (+ DeltaSeconds (`self.Tick`)))
  (if (> _returnvalue 0.01)
    (set `self.Tick` 0.0)
    (if (>= (`self.Percentage`) 101.0)
      (`self.Execute`)
      (else
        (if (== (`self.Percentage`) (`self.Last_Percentage`))
          (bind _newparam (`self.Subtract`))
          (set `self.Last_Percentage` _newparam)
          (else
            (set `self.Last_Percentage` (`self.Percentage`))))
        (`MaterialInstanceDynamic.SetScalarParameterValue` (`self.Gauge_Instance`) "Percentage" (`self.Last_Percentage`))))
    (else
      (set `self.Tick` _returnvalue))))

(fn `Add`
  (if (<= (`self.Percentage`) 101.0)
    (set `self.Percentage` (+ (`self.Percentage`) 1.0))))

(fn `Execute`)

(fn `Subtract`
  (returns (NewParam :type "Float (double-precision)"))
  (if (> (`self.Percentage`) 0.0)
    (bind _output_get (set `self.Percentage` (- (`self.Percentage`) 1.0))))
  (return _output_get))

(fn `UserConstructionScript`)