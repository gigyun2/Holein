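; UIplayer is a VR actor that drives gaze-based interaction with Menu actors.
; BeginPlay resets HMD orientation and position and makes the player controller and camera manager follow the headset.
; Tick throttles a 1500-unit debug-drawn line trace to roughly 0.02-second intervals, cast from the root component along the HMD forward vector.
; When the trace hits a Menu, it calls that actor's Add function.
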(event `self.ReceiveBeginPlay`
  (`HeadMountedDisplayFunctionLibrary.ResetOrientationAndPosition` 0.0)
  (`OculusFunctionLibrary.EnablePlayerControllerFollowHmd` true)
  (`OculusFunctionLibrary.EnablePlayerCameraManagerFollowHmd` true true))

(event `self.ReceiveActorBeginOverlap`
  (params (OtherActor :type "Actor Object Reference")))

(event `self.ReceiveTick`
  (params (DeltaSeconds :type "Float (single-precision)"))
  (bind _returnvalue (`SceneComponent.K2_GetComponentLocation` (`self.DefaultSceneRoot`)))
  (bind _returnvalue_2 (+ DeltaSeconds (`self.Tick`)))
  (if (> _returnvalue_2 0.02)
    (set `self.Tick` DeltaSeconds)
    (bind (_outhit _returnvalue_3) (`KismetSystemLibrary.LineTraceSingleForObjects` :`Start` _returnvalue :`End` (+ _returnvalue (* (`KismetMathLibrary.GetForwardVector` (`OculusFunctionLibrary.GetPose` false)) 1500.0)) :`ObjectTypes` (`|MakeArray` "ObjectTypeQuery2" "ObjectTypeQuery1" :!type "EObjectTypeQuery Enum") :`bTraceComplex` true :`DrawDebugType` "ForOneFrame"))
    (if _returnvalue_3
      (bind _asmenu (cast `/Game/Blueprint/Menu` (`.HitActor` (`GameplayStatics.BreakHitResult` _outhit))))
      (`/Game/Blueprint/Menu.Add` _asmenu))
    (else
      (set `self.Tick` _returnvalue_2))))

(fn `UserConstructionScript`)