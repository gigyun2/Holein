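; Menu_Next is a menu action actor that advances the game to the next numbered level when its Execute event fires.
; Execute splits the current level name on underscores, increments the number in the second segment, rejoins it with the first and opens that level by name.
; The scheme relies on Prefix_Number level names and does not check that the next level exists.
; BeginPlay, Tick and the construction script only call their parent versions.
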(event `self.ReceiveBeginPlay`
  (`parent.ReceiveBeginPlay`))

(event `self.ReceiveActorBeginOverlap`
  (params (OtherActor :type "Actor Object Reference")))

(event `self.ReceiveTick`
  (params (DeltaSeconds :type "Float (single-precision)"))
  (`parent.ReceiveTick` DeltaSeconds))

(event `self.Execute`
  (bind _returnvalue (`GameplayStatics.GetCurrentLevelName` true))
  (bind _returnvalue_2 (`KismetStringLibrary.ParseIntoArray` _returnvalue "_"))
  (`GameplayStatics.OpenLevel` (`KismetStringLibrary.Conv_StringToName` (`KismetStringLibrary.Concat_StrStr` (`KismetArrayLibrary.Array_Get` _returnvalue_2) "_" (`KismetStringLibrary.Conv_IntToString` (+ (`KismetStringLibrary.Conv_StringToInt` (`KismetArrayLibrary.Array_Get` _returnvalue_2 1)) 1))))))

(fn `UserConstructionScript`
  (`parent.UserConstructionScript`))